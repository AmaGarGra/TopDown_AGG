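; BP_GuardLight is a guard light that signals when the player is inside its detection Trigger.
; Trigger begin and end overlaps, filtered to CorePlayerCharacter, set DetectedPlayer, recolor SpotLight2 red or teal, and print debug taunts.
; While DetectedPlayer is true, Tick sets the light to magenta every frame, overriding the red set on entry.
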(event OnComponentBeginOverlap(Trigger)
  (params (OverlappedComponent :type Primitive%20Component%20Object%20Reference) (OtherActor :type Actor%20Object%20Reference) (OtherComp :type Primitive%20Component%20Object%20Reference) (OtherBodyIndex :type Integer) (bFromSweep :type Boolean) (SweepResult :type Hit%20Result%20Structure%20%28by%20ref%29))
  ;[1 1 1] Detecting Player
  (Utilities|Casting|CastToCorePlayerCharacter OtherActor)
  (Development|PrintString "INTRUDER!" true true "(R=1.000000,G=0.000000,B=0.041135,A=1.000000)")
  (Rendering|Components|Light|SetLightColor (Variables|Default|GetSpotLight2) "(R=0.739583,G=0.049613,B=0.236009,A=1.000000)" true)
  (Variables|Default|SetDetectedPlayer true))

(event OnComponentEndOverlap(Trigger)
  (params (OverlappedComponent :type Primitive%20Component%20Object%20Reference) (OtherActor :type Actor%20Object%20Reference) (OtherComp :type Primitive%20Component%20Object%20Reference) (OtherBodyIndex :type Integer))
  ;[1 1 1] Detecting Player
  (Utilities|Casting|CastToCorePlayerCharacter OtherActor)
  (Development|PrintString "Get back here!")
  (Rendering|Components|Light|SetLightColor (Variables|Default|GetSpotLight2) "(R=0.080220,G=0.730461,B=0.617207,A=1.000000)" true)
  (Variables|Default|SetDetectedPlayer false))

(event EventTick
  (params (DeltaSeconds :type Float%20%28single-precision%29))
  (if (Variables|Default|GetDetectedPlayer)
    (Rendering|Components|Light|SetLightColor (Variables|Default|GetSpotLight2) "(R=0.812500,G=0.065739,B=0.746396,A=1.000000)" true)))

(fn ConstructionScript)