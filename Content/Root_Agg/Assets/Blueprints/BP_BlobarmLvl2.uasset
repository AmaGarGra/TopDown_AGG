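; BP_BlobarmLvl2 is a trigger-operated door that opens only for a player character holding both blob-arm flags, Blobarm1 and Blob2.
; On overlap, the DoorOpener timeline moves the Cube between start and end positions, or a debug message asks for tentacles if either flag is missing.
; When any player character leaves the trigger, the timeline reverses to close the door.
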(event OnComponentBeginOverlap(Trigger)
  (params (OverlappedComponent :type Primitive%20Component%20Object%20Reference) (OtherActor :type Actor%20Object%20Reference) (OtherComp :type Primitive%20Component%20Object%20Reference) (OtherBodyIndex :type Integer) (bFromSweep :type Boolean) (SweepResult :type Hit%20Result%20Structure%20%28by%20ref%29))
  (bind _ascore_player_character (Utilities|Casting|CastToCorePlayerCharacter OtherActor))
  (if (and (Variables|/Game/Root_Agg/Core/Framework/CorePlayerCharacter.CorePlayerCharacter_C|GetBlobarm%201 _ascore_player_character) (Variables|/Game/Root_Agg/Core/Framework/CorePlayerCharacter.CorePlayerCharacter_C|GetBlob2 _ascore_player_character))
    (bind _newtrack_0 (Timeline|DoorOpener Play)
      (:Update
        (Transformation|SetRelativeLocation (Variables|Default|GetCube) (Math|Vector|Lerp(Vector) (Variables|Default|GetStart%20Pos) (Variables|Default|GetEnd%20Position) _newtrack_0) false false)))
    (else
      (Development|PrintString "Please insert TENTACLES"))))

(event OnComponentEndOverlap(Trigger)
  (params (OverlappedComponent :type Primitive%20Component%20Object%20Reference) (OtherActor :type Actor%20Object%20Reference) (OtherComp :type Primitive%20Component%20Object%20Reference) (OtherBodyIndex :type Integer))
  (Utilities|Casting|CastToCorePlayerCharacter OtherActor)
  (bind _newtrack_0 (Timeline|DoorOpener Reverse)
    (:Update
      (Transformation|SetRelativeLocation (Variables|Default|GetCube) (Math|Vector|Lerp(Vector) (Variables|Default|GetStart%20Pos) (Variables|Default|GetEnd%20Position) _newtrack_0) false false))))

(fn ConstructionScript)