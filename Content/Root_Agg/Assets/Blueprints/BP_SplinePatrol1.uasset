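; Spline patrol actor whose spotlight acts as a searchlight that reacts to the player.
; Each tick the SpotLight moves at constant PatrollerSpeed along the Spline in local space, jumping back to the start at the end.
; When a CorePlayerCharacter overlaps Trigger, the patrol halts, the light turns red and a debug message prints.
; When the player leaves, the light turns teal and the patrol resumes.
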(event OnComponentBeginOverlap(Trigger)
  (params (OverlappedComponent :type Primitive%20Component%20Object%20Reference) (OtherActor :type Actor%20Object%20Reference) (OtherComp :type Primitive%20Component%20Object%20Reference) (OtherBodyIndex :type Integer) (bFromSweep :type Boolean) (SweepResult :type Hit%20Result%20Structure%20%28by%20ref%29))
  ;[1 1 1] Detecting Player
  (Utilities|Casting|CastToCorePlayerCharacter OtherActor)
  (Development|PrintString "I SEE YOU!" true true "(R=1.000000,G=0.000000,B=0.041135,A=1.000000)")
  (Rendering|Components|Light|SetLightColor (Variables|Default|GetSpotLight) "(R=0.739583,G=0.049613,B=0.236009,A=1.000000)" true)
  (Variables|Default|SetDetectedPlayer true))

(event OnComponentEndOverlap(Trigger)
  (params (OverlappedComponent :type Primitive%20Component%20Object%20Reference) (OtherActor :type Actor%20Object%20Reference) (OtherComp :type Primitive%20Component%20Object%20Reference) (OtherBodyIndex :type Integer))
  ;[1 1 1] Detecting Player
  (Utilities|Casting|CastToCorePlayerCharacter OtherActor)
  (Development|PrintString "Get back here!")
  (Rendering|Components|Light|SetLightColor (Variables|Default|GetSpotLight) "(R=0.080220,G=0.730461,B=0.617207,A=1.000000)" true)
  (Variables|Default|SetDetectedPlayer false))

(event EventTick
  (params (DeltaSeconds :type Float%20%28single-precision%29))
  (bind _spline (Variables|Default|GetSpline))
  (bind _returnvalue (Spline|GetSplineLength _spline))
  ;[1 1 1] Moving on spline
  (if (not (Variables|Default|GetDetectedPlayer))
    (if (>= (Variables|Default|GetCurrentDistanceAlongSpline) _returnvalue)
      (Variables|Default|SetCurrentDistanceAlongSpline 0.0)
      (else
        (bind _output_get (Variables|Default|SetCurrentDistanceAlongSpline (Math|Interpolation|FInterptoConstant (Variables|Default|GetCurrentDistanceAlongSpline) _returnvalue DeltaSeconds (Variables|Default|GetPatrollerSpeed))))))
    (Transformation|SetRelativeLocation (Variables|Default|GetSpotLight) (Spline|GetLocationatDistanceAlongSpline _spline _output_get "Local") false false)))

(fn ConstructionScript)