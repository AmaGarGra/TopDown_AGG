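; BP_Door is a sliding door that opens for a CorePlayerCharacter who has the required tentacle arm.
; Trigger overlap scans the player's Blobarm1 array for a true entry at index BlobarmValue, printing "Need TENTACLES" for every other entry.
; A match enables input and plays the DoorOpener timeline, lerping Cube from StartPos to EndPosition.
; When the player leaves, input is disabled and the timeline reverses.
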(event OnComponentBeginOverlap(Trigger)
  (params (OverlappedComponent :type Primitive%20Component%20Object%20Reference) (OtherActor :type Actor%20Object%20Reference) (OtherComp :type Primitive%20Component%20Object%20Reference) (OtherBodyIndex :type Integer) (bFromSweep :type Boolean) (SweepResult :type Hit%20Result%20Structure%20%28by%20ref%29))
  (bind _ascore_player_character (Utilities|Casting|CastToCorePlayerCharacter OtherActor))
  (for (_array_element _array_index) (.Blobarm%201 (Variables|/Game/Root_Agg/Core/Framework/CorePlayerCharacter.CorePlayerCharacter_C|GetBlobarm%201 _ascore_player_character))
    (if (and _array_element (== _array_index (Variables|Default|GetBlobarm_value)))
      (Input|EnableInput (Game|GetPlayerController 0))
      (bind _newtrack_0 (Timeline|DoorOpener Play)
        (:Update
          (Transformation|SetRelativeLocation (Variables|Default|GetCube) (Math|Vector|Lerp(Vector) (Variables|Default|GetStart%20Pos) (Variables|Default|GetEnd%20Position) _newtrack_0) false false)))
      (else
        (Development|PrintString "Need TENTACLES" true true "(R=1.000000,G=0.000000,B=0.009549,A=1.000000)")))))

(event OnComponentEndOverlap(Trigger)
  (params (OverlappedComponent :type Primitive%20Component%20Object%20Reference) (OtherActor :type Actor%20Object%20Reference) (OtherComp :type Primitive%20Component%20Object%20Reference) (OtherBodyIndex :type Integer))
  (Utilities|Casting|CastToCorePlayerCharacter OtherActor)
  (Input|DisableInput (Game|GetPlayerController 0))
  (bind _newtrack_0 (Timeline|DoorOpener Reverse)
    (:Update
      (Transformation|SetRelativeLocation (Variables|Default|GetCube) (Math|Vector|Lerp(Vector) (Variables|Default|GetStart%20Pos) (Variables|Default|GetEnd%20Position) _newtrack_0) false false))))

(fn ConstructionScript)